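; BP_SunAndMoon is an actor that orients the Sun to match the in-game date and time.
; It caches MainGameState on BeginPlay, then each Tick feeds that state's calendar and clock, plus its own latitude, longitude and time zone, into GetSunPosition.
; The corrected elevation and azimuth become the Sun's world pitch and yaw.
; Despite the name, the graphs contain no moon logic.
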(event EventBeginPlay
  (bind _asmain_game_state (Utilities|Casting|CastToMainGameState (Game|GetGameState)))
  (Variables|Default|SetGameState _asmain_game_state))

(event EventTick
  (params (DeltaSeconds :type Float%20%28single-precision%29))
  (bind _gamestate (Variables|Default|GetGameState))
  (Utilities|IsValid (Variables|Default|GetSun)
    (:Is%20Valid
      (bind _sunpositiondata (Class|SunPositionFunctionLibrary|GetSunPosition (Variables|Default|GetLatitude) (Variables|Default|GetLongitude) (Variables|Default|GetTime%20Zone) false (Variables|/Script/FirstUnrealProject.MainGameState|GetYear _gamestate) (Variables|/Script/FirstUnrealProject.MainGameState|GetMonth _gamestate) (Variables|/Script/FirstUnrealProject.MainGameState|GetDay _gamestate) (Variables|/Script/FirstUnrealProject.MainGameState|GetHours _gamestate) (Variables|/Script/FirstUnrealProject.MainGameState|GetMinute _gamestate) (Variables|/Script/FirstUnrealProject.MainGameState|GetSecond _gamestate)))
      (Variables|Default|SetElevation (.Elevation (Utilities|Struct|BreakSunPositionData _sunpositiondata)))
      (Variables|Default|SetCorrected%20Elevation (.CorrectedElevation (Utilities|Struct|BreakSunPositionData _sunpositiondata)))
      (Variables|Default|SetAzimuth (.Azimuth (Utilities|Struct|BreakSunPositionData _sunpositiondata)))
      (Transformation|SetWorldRotation (Variables|Default|GetSun) (Math|Rotator|MakeRotator 0.0 (Variables|Default|GetCorrected%20Elevation) (Variables|Default|GetAzimuth)) false false))))

(fn ConstructionScript)