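; BP_Npc is an NPC Blueprint that manages on-screen widgets for its state.
; On BeginPlay it creates an enemy-state widget bound to its MainStateComponent and an NPC-state widget, assigning each to its own widget component.
; The HpBar event tells the stored enemy-state widget to hide HP and reset the HP bar message.
; An interaction-prompt widget setup exists but is disconnected and never runs.
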(event Custom|HpBar
  (bind _wbpnpcstate (Variables|Default|GetWBPNpcState))
  (Default|UnvisibleHp _wbpnpcstate)
  (Class|BPEnemyInterface|HpbarReSet(Message) _wbpnpcstate))

(event EventBeginPlay
  (bind _returnvalue (UserInterface|CreateWidget "/Game/UI/State/WBP_EnemyState.WBP_EnemyState_C" 0 (Variables|Default|GetMainStateComponent)))
  (UserInterface|SetWidget (Variables|Default|GetWidgetComponent) _returnvalue)
  (Variables|Default|SetWBPNpcState _returnvalue)
  (bind _returnvalue_2 (UserInterface|CreateWidget "/Game/UI/State/WBP_NpcState.WBP_NpcState_C"))
  (UserInterface|SetWidget (Variables|Default|GetNpcWidgetComponent) _returnvalue_2))

(fn ConstructionScript)