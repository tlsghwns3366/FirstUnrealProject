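; BP_Sun is a Blueprint meant to orient a Sun object by real solar position for the game's date and time.
; On BeginPlay it caches MainGameState, whose date and clock, with latitude, longitude and time zone, would feed GetSunPosition to set rotation from corrected elevation and azimuth.
; That update logic is disconnected and never runs, and Tick is empty, so the Sun is not moved by this graph.
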(event EventBeginPlay
  (bind _asmain_game_state (Utilities|Casting|CastToMainGameState (Game|GetGameState)))
  (Variables|Default|SetGameState _asmain_game_state))

(event EventTick
  (params (DeltaSeconds :type Float%20%28single-precision%29)))

(fn ConstructionScript)