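; AI controller for enemy minions that turns perception updates into Blackboard state.
; Each update stores the stimulus location, sets FindTarget, and sets Target to the perceived actor when sensed or AddDamage is true, clearing it otherwise.
; DoOnce gates record the pawn's location as StartPosition on BeginPlay and again on the first perception update.
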(event OnTargetPerceptionUpdated(AIPerceptionComponent)
  (params (Actor :type Actor%20Object%20Reference) (Stimulus :type AI%20Stimulus%20Structure))
  (bind (_age _expirationage _strength _stimuluslocation _receiverlocation _tag _bsuccessfullysensed) (Utilities|Struct|BreakAIStimulus Stimulus))
  (AI|Components|Blackboard|SetValueasObject (Variables|Default|GetBlackboard) (Utilities|Name|MakeLiteralName "Target") (Utilities|SelectObject Actor 0 (or _bsuccessfullysensed (Variables|Default|GetAddDamage))))
  (AI|Components|Blackboard|SetValueasVector (Variables|Default|GetBlackboard) (Utilities|Name|MakeLiteralName "LastSenseLocation") _stimuluslocation)
  (AI|Components|Blackboard|SetValueasBool (Variables|Default|GetBlackboard) (Utilities|Name|MakeLiteralName "FindTarget") true)
  (Utilities|FlowControl|DoOnce false
    (:Completed
      (AI|Components|Blackboard|SetValueasVector (Variables|Default|GetBlackboard) (Utilities|Name|MakeLiteralName "StartPosition") (Transformation|GetActorLocation (Pawn|GetControlledPawn))))))

(event EventBeginPlay
  (Utilities|FlowControl|DoOnce false
    (:Completed
      (AI|Components|Blackboard|SetValueasVector (Variables|Default|GetBlackboard) (Utilities|Name|MakeLiteralName "StartPosition") (Transformation|GetActorLocation (Pawn|GetControlledPawn))))))

(fn ConstructionScript)