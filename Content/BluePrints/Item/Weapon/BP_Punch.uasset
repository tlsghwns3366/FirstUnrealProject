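; Punch weapon Blueprint that alternates its StaticMesh between the left and right hand across a four-step combo.
; BeginPlay attaches the mesh to the SceneComponent, and WeaponInitialize resets the combo counter.
; Each WeaponAction re-attaches the mesh to the left or right weapon socket on AttachMesh by combo step, then advances the counter, wrapping after the last step.
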(event EventBeginPlay
  (Transformation|AttachComponentToComponent (Variables|Default|GetStaticMesh) (Variables|Default|GetSceneComponent) "None" "KeepRelative" "KeepRelative" "KeepRelative" true))

(event EventWeaponAction
  (switch int (Variables|Default|GetAttackCombo)
    (:0
      (Transformation|AttachComponentToComponent (Variables|Default|GetStaticMesh) (Variables|Default|GetAttachMesh) "WeaponSocket_L" "KeepRelative" "KeepRelative" "KeepRelative" true :!label _label))
    (:1
      (Transformation|AttachComponentToComponent (Variables|Default|GetStaticMesh) (Variables|Default|GetAttachMesh) "WeaponSocket_R" "KeepRelative" "KeepRelative" "KeepRelative" true :!label _label_2))
    (:2
      (goto _label))
    (:3
      (goto _label_2)))
  (bind _result (Math|Integer|IncrementInt (Variables|Default|GetAttackCombo))
    (:%20%20
      (if (> _result 3)
        (Variables|Default|SetAttackCombo 0)
        (else
          (Variables|Default|SetAttackCombo _result))))))

(event EventWeaponInitialize
  (Variables|Default|SetAttackCombo 0))

(fn ConstructionScript)