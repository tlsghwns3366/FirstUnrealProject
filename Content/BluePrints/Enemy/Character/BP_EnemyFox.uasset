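; BP_EnemyFox is a fox enemy character that extends a parent enemy Blueprint with its own bite actor, movement speeds and hit reaction.
; On BeginPlay it spawns BP_BiteFox and attaches it to the mesh's AttackSocket.
; ChangeState sets walk speed for the Find, Rest or Idle state and updates the rest flag on the EnemyAnimInstance.
; AnyDamage plays a hit montage unless the fox is attacking.
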(event EventBeginPlay
  (|CallParentFunction)
  (bind _returnvalue (Game|SpawnActorfromClass "/Game/BluePrints/Item/Weapon/BP_BiteFox.BP_BiteFox_C" (Transformation|GetSocketTransform (Variables|Character|GetMesh) "AttackSocket" "RTS_World") "Undefined" "MultiplyWithRoot" 0 0))
  (Transformation|AttachComponentToComponent _returnvalue (Variables|Character|GetMesh) "AttackSocket" "SnapToTarget" "SnapToTarget" "KeepRelative" true))

(event EventChangeState
  (params (EnemyState :type E_EnemyState%20Enum :default "NewEnumerator0"))
  (Variables|Default|SetEnemy%20State EnemyState)
  (Variables|/Script/Engine.CharacterMovementComponent|SetMaxWalkSpeed (Variables|Character|GetCharacterMovement) (Utilities|Select :Index (Variables|Default|GetEnemy%20State) :NewEnumerator0 3e+02 :NewEnumerator1 0.0 :NewEnumerator2 2e+02))
  (bind _asenemy_anim_instance (Utilities|Casting|CastToEnemyAnimInstance (Components|SkeletalMesh|GetAnimInstance (Variables|Character|GetMesh))))
  (Variables|/Script/FirstUnrealProject.EnemyAnimInstance|SetIsRest _asenemy_anim_instance (Utilities|Select :Index (Variables|Default|GetEnemy%20State) :NewEnumerator0 false :NewEnumerator1 true :NewEnumerator2 false)))

(event Game|Damage|EventAnyDamage
  (params (Damage :type Float%20%28single-precision%29) (DamageType :type Damage%20Type%20Object%20Reference) (InstigatedBy :type Controller%20Object%20Reference) (DamageCauser :type Actor%20Object%20Reference))
  (Utilities|FlowControl|Sequence
    (:then_0
      (if (not (Variables|Default|GetIsAttacking))
        (Animation|Montage|PlayMontage (Variables|Character|GetMesh) "/Game/Animation/Enemy/Fox/AM_EnemyFoxHit.AM_EnemyFoxHit" 1.0 0.0 "Default")))))

(fn ConstructionScript
  (|CallParentFunction))