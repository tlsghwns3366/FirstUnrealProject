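; Enemy Blueprint that provides the enemy's state display and a toggleable inventory screen.
; BeginPlay creates a state widget from the state component and assigns it to the Widget component; Hpbar calls its hide and reset functions.
; SetEnemyInventory opens an inventory widget bound to this enemy with mouse cursor and Game-and-UI input.
; The next call runs GetAllItem, removes the widget and restores game-only input.
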(event Custom|Hpbar
  (bind _wbpenemystate (Variables|Default|GetWBPEnemyState))
  (Default|UnvisibleHp _wbpenemystate)
  (Class|BPEnemyInterface|HpbarReSet(Message) _wbpenemystate))

(event EventBeginPlay
  (bind _returnvalue (UserInterface|CreateWidget "/Game/UI/WBP_EnemyState.WBP_EnemyState_C" 0 (Variables|Default|GetEnemyStateComponent)))
  (UserInterface|SetWidget (Variables|Default|GetWidget) _returnvalue)
  (Variables|Default|SetWBPEnemyState _returnvalue))

(event EventSetEnemyInventory
  (bind _returnvalue (Game|GetPlayerController 0))
  (bind _returnvalue_2 (Game|GetPlayerController 0))
  (if (not (Variables|Default|GetInventoryOpen))
    (Variables|Default|SetInventoryOpen true)
    (bind _returnvalue_3 (UserInterface|CreateWidget "/Game/UI/WBP_EnemyInventory.WBP_EnemyInventory_C"))
    (bind _output_get (Variables|Default|SetWBPEnemyInventory _returnvalue_3))
    (Variables|/Game/UI/WBP_EnemyInventory.WBP_EnemyInventory_C|SetEnemyInventory _output_get (Variables|Default|GetEnemyInventoryComponent))
    (Default|InitializeBind (Variables|Default|GetWBPEnemyInventory) self)
    (UserInterface|Viewport|AddtoViewport (Variables|Default|GetWBPEnemyInventory) 0)
    (Variables|/Script/Engine.PlayerController|SetbShowMouseCursor _returnvalue_2 true)
    (Input|SetInputModeGameandUI _returnvalue_2 0 "DoNotLock" true false)
    (else
      (Variables|Default|SetInventoryOpen false)
      (Default|GetAllItem (Variables|Default|GetWBPEnemyInventory))
      (Widget|RemovefromParent (Variables|Default|GetWBPEnemyInventory))
      (Variables|/Script/Engine.PlayerController|SetbShowMouseCursor _returnvalue false)
      (Input|SetInputModeGameOnly _returnvalue false))))

(fn ConstructionScript)