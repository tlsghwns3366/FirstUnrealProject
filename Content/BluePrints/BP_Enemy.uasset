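; BP_Enemy is an enemy Blueprint that exposes its inventory to the player through a toggleable UI.
; SetEnemyInventory flips InventoryOpen, creating a new WBP_EnemyInventory widget wired to EnemyInventoryComponent and bound to this enemy, or removing it.
; Opening shows the mouse cursor with Game and UI input; closing hides it and restores game-only input.
; The event has no caller in this graph.
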(event EventBeginPlay)

(event Collision|EventActorBeginOverlap
  (params (OtherActor :type Actor%20Object%20Reference)))

(event EventTick
  (params (DeltaSeconds :type Float%20%28single-precision%29)))

(event EventSetEnemyInventory
  (bind _returnvalue (Game|GetPlayerController 0))
  (bind _returnvalue_2 (Game|GetPlayerController 0))
  (if (not (Variables|Default|GetInventoryOpen))
    (Variables|Default|SetInventoryOpen true)
    (bind _returnvalue_3 (UserInterface|CreateWidget "/Game/UI/WBP_EnemyInventory.WBP_EnemyInventory_C"))
    (bind _output_get (Variables|Default|SetWBPEnemyInventory _returnvalue_3))
    (Variables|/Game/UI/WBP_EnemyInventory.WBP_EnemyInventory_C|SetEnemyInventory _output_get (Variables|Default|GetEnemyInventoryComponent))
    (Default|InitializeBind (Variables|Default|GetWBPEnemyInventory) self)
    (UserInterface|Viewport|AddtoViewport (Variables|Default|GetWBPEnemyInventory) 0)
    (Variables|/Script/Engine.PlayerController|SetbShowMouseCursor _returnvalue_2 true)
    (Input|SetInputModeGameandUI _returnvalue_2 0 "DoNotLock" true false)
    (else
      (Variables|Default|SetInventoryOpen false)
      (Widget|RemovefromParent (Variables|Default|GetWBPEnemyInventory))
      (Variables|/Script/Engine.PlayerController|SetbShowMouseCursor _returnvalue false)
      (Input|SetInputModeGameOnly _returnvalue false))))

(fn ConstructionScript)